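; BP_MushroomLight is a glowing-mushroom prop actor, filed under cave generation, that varies its look at runtime.
; On BeginPlay it picks a random integer and switches the Mushroom component to one of nine LightMushroom static meshes.
; The random range has ten values for nine cases, so one roll leaves the component's default mesh in place.
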(event EventBeginPlay
  (bind _mushroom (Variables|Default|GetMushroom))
  (switch int (Math|Random|RandomIntegerinRange 0 9)
    (:0
      (Components|StaticMesh|SetStaticMesh _mushroom "/Game/LuosCaves/Meshes/Props_Mushrooms/SM_LProp_Free_LightMushroom_01.SM_LProp_Free_LightMushroom_01"))
    (:1
      (Components|StaticMesh|SetStaticMesh _mushroom "/Game/LuosCaves/Meshes/Props_Mushrooms/SM_LProp_Free_LightMushroom_02.SM_LProp_Free_LightMushroom_02"))
    (:2
      (Components|StaticMesh|SetStaticMesh _mushroom "/Game/LuosCaves/Meshes/Props_Mushrooms/SM_LProp_Free_LightMushroom_03.SM_LProp_Free_LightMushroom_03"))
    (:3
      (Components|StaticMesh|SetStaticMesh _mushroom "/Game/LuosCaves/Meshes/Props_Mushrooms/SM_LProp_Free_LightMushroom_04.SM_LProp_Free_LightMushroom_04"))
    (:4
      (Components|StaticMesh|SetStaticMesh _mushroom "/Game/LuosCaves/Meshes/Props_Mushrooms/SM_LProp_Free_LightMushroom_05.SM_LProp_Free_LightMushroom_05"))
    (:5
      (Components|StaticMesh|SetStaticMesh _mushroom "/Game/LuosCaves/Meshes/Props_Mushrooms/SM_LProp_Free_LightMushroom_06.SM_LProp_Free_LightMushroom_06"))
    (:6
      (Components|StaticMesh|SetStaticMesh _mushroom "/Game/LuosCaves/Meshes/Props_Mushrooms/SM_LProp_Free_LightMushroom_07.SM_LProp_Free_LightMushroom_07"))
    (:7
      (Components|StaticMesh|SetStaticMesh _mushroom "/Game/LuosCaves/Meshes/Props_Mushrooms/SM_LProp_Free_LightMushroom_08.SM_LProp_Free_LightMushroom_08"))
    (:8
      (Components|StaticMesh|SetStaticMesh _mushroom "/Game/LuosCaves/Meshes/Props_Mushrooms/SM_LProp_Free_LightMushroom_09.SM_LProp_Free_LightMushroom_09"))))

(event Collision|EventActorBeginOverlap
  (params (OtherActor :type Actor%20Object%20Reference)))

(event EventTick
  (params (DeltaSeconds :type Float%20%28single-precision%29)))

(fn ConstructionScript)