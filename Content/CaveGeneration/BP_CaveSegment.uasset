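; Procedural cave segment actor that shapes itself into a straight, corner, T, crossroad or dead-end piece from its open door directions.
; The construction script uses fixed doors or randomly adds unbanned directions to the required ones.
; SetMeshForDirections picks and rotates the mesh, reveals matching decor and destroys tagged meshes of other shapes.
; BeginPlay randomly spawns scaled mushroom lights at the shape's tagged arrows and randomly yaws "rotatable" meshes.
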(event EventBeginPlay
  (for _array_element (Actor|GetComponentsbyTag "/Script/Engine.ArrowComponent" (Utilities|String|StringToName (Variables|Default|GetMushroom%20Tag)))
    (if (== (Math|Random|RandomIntegerinRange 0 1) 0)
      (bind _returnvalue (Game|SpawnActorfromClass "/Game/CaveGeneration/BP_MushroomLight.BP_MushroomLight_C" (Math|Transform|MakeTransform (.location (Transformation|GetWorldTransform _array_element)) (Math|Rotator|MakeRotator (.roll (Variables|/Script/Engine.SceneComponent|GetRelativeRotation _array_element)) (.pitch (Variables|/Script/Engine.SceneComponent|GetRelativeRotation _array_element)) (.yaw (Variables|/Script/Engine.SceneComponent|GetRelativeRotation _array_element))) (Math|Vector|MakeVector (+ (.x (.scale (Transformation|GetWorldTransform _array_element))) (Math|Random|RandomFloatinRange 0.0 1.5)) (+ (.y (.scale (Transformation|GetWorldTransform _array_element))) (Math|Random|RandomFloatinRange 0.0 1.5)) (+ (.z (.scale (Transformation|GetWorldTransform _array_element))) (Math|Random|RandomFloatinRange 0.0 1.5)))) "Undefined" 0 0))
      (Transformation|SetActorRelativeRotation _returnvalue "0.000000, 0, 0")))
  (for _array_element_2 (Actor|GetComponentsbyTag "/Script/Engine.StaticMeshComponent" "rotatable")
    (Transformation|AddRelativeRotation _array_element_2 (Math|Rotator|MakeRotator 0.0 0.0 (Math|Random|RandomFloatinRange 0.0 3.6e+02)) false false)))

(event Collision|EventActorBeginOverlap
  (params (OtherActor :type Actor%20Object%20Reference)))

(event EventTick
  (params (DeltaSeconds :type Float%20%28single-precision%29)))

(fn ConstructionScript
  (if (Variables|Default|GetHasFixedDoors)
    (Variables|Default|SetDirections%20To%20Use (Variables|Default|GetDoor%20Directions))
    (else
      (bind _door_directions (CallFunction|GetDirectionsReqandRes (Variables|Default|GetMinimumDoorDirections) (Variables|Default|GetRestrictedDoorDirections)))
      (Variables|Default|SetDirections%20To%20Use _door_directions)))
  (CallFunction|SetMeshforDirections (Variables|Default|GetDirections%20To%20Use)))

(fn GetDirectionsReqandRes
  (params (Required :type Array%20of%20Enum_Directions%20Enums) (Banned :type Array%20of%20Enum_Directions%20Enums))
  (LocalVariables|SetRequired%20directions Required)
  (LocalVariables|SetRestricted%20Directions Banned)
  (bind _enumvalue (|ForEachEnum_Directions)
    (:LoopBody
      (if (Utilities|Array|ContainsItem (LocalVariables|GetRequired%20directions) _enumvalue) ; Is explicitly required
        (Utilities|Array|Add (LocalVariables|GetOutput%20Directions) _enumvalue)
        (Variables|Default|SetDoor%20Directions (LocalVariables|GetOutput%20Directions) :!label _label)
        (elif (not (Utilities|Array|ContainsItem (LocalVariables|GetRestricted%20Directions) _enumvalue)) ; is explicitly banned
          (if (== (Math|Random|RandomInteger 3) 0)
            (Utilities|Array|Add (LocalVariables|GetOutput%20Directions) _enumvalue)
            (goto _label)))))
    (:then
      (return (LocalVariables|GetOutput%20Directions)))))

(fn SetMeshforDirections
  (params (OpenDoors :type Array%20of%20Enum_Directions%20Enums))
  (bind _x_decour (Variables|Default|GetX%20Decour))
  (LocalVariables|SetDoors%20That%20Are%20Open OpenDoors)
  (if false
    (Components|StaticMesh|SetStaticMesh (Variables|Default|GetCavePiece) "/Game/LuosCaves/Meshes/Caves_LSections/SM_LCave_Free_CHL_01.SM_LCave_Free_CHL_01")
    (elif (Math|Boolean|ANDBoolean (Utilities|Array|ContainsItem (LocalVariables|GetDoors%20That%20Are%20Open) "NewEnumerator2") (Utilities|Array|ContainsItem (LocalVariables|GetDoors%20That%20Are%20Open) "NewEnumerator3") (== (Utilities|Array|Length (LocalVariables|GetDoors%20That%20Are%20Open)) 2)) ; Horizontal
      (Components|StaticMesh|SetStaticMesh (Variables|Default|GetCavePiece) "/Game/LuosCaves/Meshes/Caves_ISections/SM_LCave_Free_CHI_01.SM_LCave_Free_CHI_01")
      (Transformation|AddRelativeRotation (Variables|Default|GetCenter) "0,90.000000, 0" false false)
      (Rendering|SetVisibility (Variables|Default|GetI%20Decour) true true :!label _label)
      (Variables|Default|SetMushroom%20Tag "i")
      (Utilities|TurnOffCollisionforTag "lm"
        (:Completed
          (Utilities|TurnOffCollisionforTag "tm"
            (:Completed
              (Utilities|TurnOffCollisionforTag "xm")))))
      (elif (Math|Boolean|ANDBoolean (Utilities|Array|ContainsItem (LocalVariables|GetDoors%20That%20Are%20Open) "NewEnumerator0") (Utilities|Array|ContainsItem (LocalVariables|GetDoors%20That%20Are%20Open) "NewEnumerator1") (== (Utilities|Array|Length (LocalVariables|GetDoors%20That%20Are%20Open)) 2)) ; Vertical
        (Components|StaticMesh|SetStaticMesh (Variables|Default|GetCavePiece) "/Game/LuosCaves/Meshes/Caves_ISections/SM_LCave_Free_CHI_01.SM_LCave_Free_CHI_01")
        (goto _label)
        (elif (Math|Boolean|ANDBoolean (Utilities|Array|ContainsItem (LocalVariables|GetDoors%20That%20Are%20Open) "NewEnumerator2") (Utilities|Array|ContainsItem (LocalVariables|GetDoors%20That%20Are%20Open) "NewEnumerator3") (Utilities|Array|ContainsItem (LocalVariables|GetDoors%20That%20Are%20Open) "NewEnumerator0") (Utilities|Array|ContainsItem (LocalVariables|GetDoors%20That%20Are%20Open) "NewEnumerator1"))
          (Components|StaticMesh|SetStaticMesh (Variables|Default|GetCavePiece) "/Game/LuosCaves/Meshes/Caves_XSections/SM_LCave_Free_CRX_01.SM_LCave_Free_CRX_01")
          (Transformation|AddRelativeRotation (Variables|Default|GetCenter) (Math|Rotator|MakeRotator 0.0 0.0 (* (Math|Random|RandomIntegerinRange 0 4) 9e+01)) false false)
          (Rendering|SetVisibility _x_decour true true)
          (Variables|Default|SetMushroom%20Tag "x")
          (Collision|SetCollisionEnabled _x_decour "NoCollision")
          (Utilities|TurnOffCollisionforTag "lm"
            (:Completed
              (Utilities|TurnOffCollisionforTag "tm"
                (:Completed
                  (Utilities|TurnOffCollisionforTag "im")))))
          (elif (Math|Boolean|ANDBoolean (Utilities|Array|ContainsItem (LocalVariables|GetDoors%20That%20Are%20Open) "NewEnumerator0") (Utilities|Array|ContainsItem (LocalVariables|GetDoors%20That%20Are%20Open) "NewEnumerator2") (== (Utilities|Array|Length (LocalVariables|GetDoors%20That%20Are%20Open)) 2)) ; L
            (Components|StaticMesh|SetStaticMesh (Variables|Default|GetCavePiece) "/Game/LuosCaves/Meshes/Caves_LSections/SM_LCave_Free_CHL_01.SM_LCave_Free_CHL_01")
            (Transformation|AddRelativeRotation (Variables|Default|GetCenter) "0,180.000000, 0" false false)
            (Rendering|SetVisibility (Variables|Default|GetL%20Decour) true true :!label _label_2)
            (Variables|Default|SetMushroom%20Tag "l")
            (Utilities|TurnOffCollisionforTag "im"
              (:Completed
                (Utilities|TurnOffCollisionforTag "tm"
                  (:Completed
                    (Utilities|TurnOffCollisionforTag "xm")))))
            (elif (Math|Boolean|ANDBoolean (Utilities|Array|ContainsItem (LocalVariables|GetDoors%20That%20Are%20Open) "NewEnumerator2") (Utilities|Array|ContainsItem (LocalVariables|GetDoors%20That%20Are%20Open) "NewEnumerator1") (== (Utilities|Array|Length (LocalVariables|GetDoors%20That%20Are%20Open)) 2)) ; L
              (Components|StaticMesh|SetStaticMesh (Variables|Default|GetCavePiece) "/Game/LuosCaves/Meshes/Caves_LSections/SM_LCave_Free_CHL_01.SM_LCave_Free_CHL_01")
              (Transformation|AddRelativeRotation (Variables|Default|GetCenter) "0,270.000000, 0" false false)
              (goto _label_2)
              (elif (Math|Boolean|ANDBoolean (Utilities|Array|ContainsItem (LocalVariables|GetDoors%20That%20Are%20Open) "NewEnumerator1") (Utilities|Array|ContainsItem (LocalVariables|GetDoors%20That%20Are%20Open) "NewEnumerator3") (== (Utilities|Array|Length (LocalVariables|GetDoors%20That%20Are%20Open)) 2)) ; L
                (Components|StaticMesh|SetStaticMesh (Variables|Default|GetCavePiece) "/Game/LuosCaves/Meshes/Caves_LSections/SM_LCave_Free_CHL_01.SM_LCave_Free_CHL_01")
                (Transformation|AddRelativeRotation (Variables|Default|GetCenter) "0,0.000000, 0" false false)
                (goto _label_2)
                (elif (Math|Boolean|ANDBoolean (Utilities|Array|ContainsItem (LocalVariables|GetDoors%20That%20Are%20Open) "NewEnumerator3") (Utilities|Array|ContainsItem (LocalVariables|GetDoors%20That%20Are%20Open) "NewEnumerator0") (== (Utilities|Array|Length (LocalVariables|GetDoors%20That%20Are%20Open)) 2)) ; L
                  (Components|StaticMesh|SetStaticMesh (Variables|Default|GetCavePiece) "/Game/LuosCaves/Meshes/Caves_LSections/SM_LCave_Free_CHL_01.SM_LCave_Free_CHL_01")
                  (Transformation|AddRelativeRotation (Variables|Default|GetCenter) "0,90.000000, 0" false false)
                  (goto _label_2)
                  (elif (and (not (Utilities|Array|ContainsItem (LocalVariables|GetDoors%20That%20Are%20Open) "NewEnumerator3")) (== (Utilities|Array|Length (LocalVariables|GetDoors%20That%20Are%20Open)) 3)) ; T
                    (Components|StaticMesh|SetStaticMesh (Variables|Default|GetCavePiece) "/Game/LuosCaves/Meshes/Caves_Tsections/SM_LCave_Free_CRT_01.SM_LCave_Free_CRT_01")
                    (Transformation|AddRelativeRotation (Variables|Default|GetCenter) "0,270.000000, 0" false false)
                    (Rendering|SetVisibility (Variables|Default|GetT%20Decour) true true :!label _label_3)
                    (Variables|Default|SetMushroom%20Tag "t")
                    (Utilities|TurnOffCollisionforTag "lm"
                      (:Completed
                        (Utilities|TurnOffCollisionforTag "lm"
                          (:Completed
                            (Utilities|TurnOffCollisionforTag "xm")))))
                    (elif (and (not (Utilities|Array|ContainsItem (LocalVariables|GetDoors%20That%20Are%20Open) "NewEnumerator0")) (== (Utilities|Array|Length (LocalVariables|GetDoors%20That%20Are%20Open)) 3)) ; T
                      (Components|StaticMesh|SetStaticMesh (Variables|Default|GetCavePiece) "/Game/LuosCaves/Meshes/Caves_Tsections/SM_LCave_Free_CRT_01.SM_LCave_Free_CRT_01")
                      (Transformation|AddRelativeRotation (Variables|Default|GetCenter) "0,0.000000, 0" false false)
                      (goto _label_3)
                      (elif (and (not (Utilities|Array|ContainsItem (LocalVariables|GetDoors%20That%20Are%20Open) "NewEnumerator2")) (== (Utilities|Array|Length (LocalVariables|GetDoors%20That%20Are%20Open)) 3)) ; T
                        (Components|StaticMesh|SetStaticMesh (Variables|Default|GetCavePiece) "/Game/LuosCaves/Meshes/Caves_Tsections/SM_LCave_Free_CRT_01.SM_LCave_Free_CRT_01")
                        (Transformation|AddRelativeRotation (Variables|Default|GetCenter) "0,90.000000, 0" false false)
                        (goto _label_3)
                        (elif (and (not (Utilities|Array|ContainsItem (LocalVariables|GetDoors%20That%20Are%20Open) "NewEnumerator1")) (== (Utilities|Array|Length (LocalVariables|GetDoors%20That%20Are%20Open)) 3)) ; T
                          (Components|StaticMesh|SetStaticMesh (Variables|Default|GetCavePiece) "/Game/LuosCaves/Meshes/Caves_Tsections/SM_LCave_Free_CRT_01.SM_LCave_Free_CRT_01")
                          (Transformation|AddRelativeRotation (Variables|Default|GetCenter) "0,180.000000, 0" false false)
                          (goto _label_3)
                          (elif (and (Utilities|Array|ContainsItem (LocalVariables|GetDoors%20That%20Are%20Open) "NewEnumerator3") (== (Utilities|Array|Length (LocalVariables|GetDoors%20That%20Are%20Open)) 1)) ; Dead End
                            (Components|StaticMesh|SetStaticMesh (Variables|Default|GetCavePiece) "/Game/LuosCaves/Meshes/Caves_LSections/SM_LCave_Free_CHL_01.SM_LCave_Free_CHL_01")
                            (Transformation|AddRelativeRotation (Variables|Default|GetCenter) "0,90.000000, 0" false false)
                            (Rendering|SetVisibility (Variables|Default|GetDeadEndRock) true false :!label _label_4)
                            (Rendering|SetVisibility (Variables|Default|GetL%20Decour) true true)
                            (Variables|Default|SetMushroom%20Tag "l")
                            (Utilities|TurnOffCollisionforTag "im"
                              (:Completed
                                (Utilities|TurnOffCollisionforTag "tm"
                                  (:Completed
                                    (Utilities|TurnOffCollisionforTag "xm")))))
                            (elif (and (Utilities|Array|ContainsItem (LocalVariables|GetDoors%20That%20Are%20Open) "NewEnumerator0") (== (Utilities|Array|Length (LocalVariables|GetDoors%20That%20Are%20Open)) 1)) ; Dead End
                              (Components|StaticMesh|SetStaticMesh (Variables|Default|GetCavePiece) "/Game/LuosCaves/Meshes/Caves_LSections/SM_LCave_Free_CHL_01.SM_LCave_Free_CHL_01")
                              (Transformation|AddRelativeRotation (Variables|Default|GetCenter) "0,180.000000, 0" false false)
                              (goto _label_4)
                              (elif (and (Utilities|Array|ContainsItem (LocalVariables|GetDoors%20That%20Are%20Open) "NewEnumerator2") (== (Utilities|Array|Length (LocalVariables|GetDoors%20That%20Are%20Open)) 1)) ; Dead End
                                (Components|StaticMesh|SetStaticMesh (Variables|Default|GetCavePiece) "/Game/LuosCaves/Meshes/Caves_LSections/SM_LCave_Free_CHL_01.SM_LCave_Free_CHL_01")
                                (Transformation|AddRelativeRotation (Variables|Default|GetCenter) "0,270.000000, 0" false false)
                                (goto _label_4)
                                (elif (and (Utilities|Array|ContainsItem (LocalVariables|GetDoors%20That%20Are%20Open) "NewEnumerator1") (== (Utilities|Array|Length (LocalVariables|GetDoors%20That%20Are%20Open)) 1)) ; Dead end
                                  (Components|StaticMesh|SetStaticMesh (Variables|Default|GetCavePiece) "/Game/LuosCaves/Meshes/Caves_LSections/SM_LCave_Free_CHL_01.SM_LCave_Free_CHL_01")
                                  (Transformation|AddRelativeRotation (Variables|Default|GetCenter) "0,0.000000, 0" false false)
                                  (goto _label_4))))))))))))))))))