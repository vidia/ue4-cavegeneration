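; BP_CaveParent is a base cave segment actor for cave generation that rotates itself to fit the door directions required at its location.
; The construction script compares relative and desired door directions, yawing 90 degrees up to three times until they match, logging an error otherwise.
; Each turn appends remapped directions rather than replacing them, and the clockwise helper maps SOUTH to itself and EAST to WEST.
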(event EventBeginPlay)

(event Collision|EventActorBeginOverlap
  (params (OtherActor :type Actor%20Object%20Reference)))

(event EventTick
  (params (DeltaSeconds :type Float%20%28single-precision%29)))

(fn ConstructionScript
  (CallFunction|RotateSelftoMatchDoors (Variables|Default|GetRelative%20Door%20Directions) (Variables|Default|GetDesired%20World%20Door%20Directions)))

(fn RotateSelftoMatchDoors
  (params (Relative%20Door%20Directions :type Array%20of%20Enum_Directions%20Enums) (World%20Door%20Directions :type Array%20of%20Enum_Directions%20Enums))
  (LocalVariables|SetLocal%20World%20Door%20Directions World%20Door%20Directions)
  (bind _match (CallFunction|DirectionArraysMatch Relative%20Door%20Directions World%20Door%20Directions))
  (if _match
    (return)
    (else
      (LocalVariables|SetNew%20Relative%20Doors Relative%20Door%20Directions)
      (for _index (range 1 3)
        (Class|Actor|AddActorWorldRotation "0,90.000000, 0")
        (for _array_element (LocalVariables|GetNew%20Relative%20Doors)
          (bind _output (CallFunction|RotateDirectionClockwise _array_element))
          (Utilities|Array|Add (LocalVariables|GetNew%20Relative%20Doors) _output))
        (bind _match_2 (CallFunction|DirectionArraysMatch (LocalVariables|GetNew%20Relative%20Doors) (LocalVariables|GetLocal%20World%20Door%20Directions)))
        (if _match_2
          (return)))
      ;[1 0.5048 0.01547] This is an error. Handle this better
      (Development|PrintString "The Cave Segment can't fit the requirements for this location." false true "(R=1.000000,G=0.008232,B=0.000000,A=1.000000)" 5.0)
      (return))))

(fn RotateDirectionClockwise
  (params (Input :type Enum_Directions%20Enum))
  (switch Utilities|FlowControl|Switch|SwitchonEnum_Directions Input
    (:NewEnumerator0
      (LocalVariables|SetTo%20Return "NewEnumerator2"))
    (:NewEnumerator1
      (LocalVariables|SetTo%20Return "NewEnumerator1"))
    (:NewEnumerator2
      (LocalVariables|SetTo%20Return "NewEnumerator3"))
    (:NewEnumerator3
      (LocalVariables|SetTo%20Return "NewEnumerator0")))
  (return (LocalVariables|GetTo%20Return)))

(fn DirectionArraysMatch
  (params (One :type Array%20of%20Enum_Directions%20Enums) (Two :type Array%20of%20Enum_Directions%20Enums))
  (if (== (Utilities|Array|Length One) (Utilities|Array|Length Two))
    (bind _array_element (Utilities|Array|ForEachLoopwithBreak One :!label _label)
      (:LoopBody
        (if (not (Utilities|Array|ContainsItem Two _array_element))
          (LocalVariables|SetDoMatch false)
          (goto _label Break)))
      (:Completed
        (return (LocalVariables|GetDoMatch))))
    (else
      (return false))))